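; Motion_BP is a motion comparator Blueprint that defines a motion from an editable array of points, which must hold at least two.
; InitializeComponents passes a reference component and four motion points to Initialize.
; The completion and failure events each print a debug message and destroy the actor.
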(event EventBeginPlay)

(event EventOnMotionComplete
  (Development|PrintString "Motion Complete Event Triggered")
  (Actor|DestroyActor))

(event EventOnMotionFailed
  (Development|PrintString "Motion Failed Event Triggered")
  (Actor|DestroyActor))

(fn ConstructionScript)

(fn InitializeComponents
  (params (ComponentReference :type Primitive%20Component%20Object%20Reference))
  (Class|Motion|Initialize ComponentReference (Utilities|Array|MakeArray (Variables|Default|GetMotionPoint_0) (Variables|Default|GetMotionPoint_1) (Variables|Default|GetMotionPoint_2) (Variables|Default|GetMotionPoint_3))))